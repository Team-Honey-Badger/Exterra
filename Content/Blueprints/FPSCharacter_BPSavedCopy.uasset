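; First-person player character that handles attack input, damage and death.
; On begin play it adds the GameHUD widget to the viewport; left mouse toggles IsAttacking and makes noise at the player's location on press.
; Damage plays a sound and drains Health until death, which calls Kill, disables movement, hides the first-person mesh and shows the body mesh, with physics simulation enabled on both.
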(event EventBeginPlay
  ;[1 1 1] Attach HUD to player's viewport
  (|CallParentFunction)
  (bind _returnvalue (UserInterface|CreateWidget "/Game/UMG/GameHUD.GameHUD_C" (Game|GetPlayerController 0)))
  (UserInterface|Viewport|AddtoViewport _returnvalue 0)
  (Actor|Tick|SetActorTickEnabled true))

(event EventAnyDamage
  (params (Damage :type Float%20%28single-precision%29) (DamageType :type Damage%20Type%20Object%20Reference) (InstigatedBy :type Controller%20Object%20Reference) (DamageCauser :type Actor%20Object%20Reference))
  (bind _firstpersonmesh (Variables|Default|GetFirstPersonMesh))
  (bind _mesh (Variables|Character|GetMesh))
  (if (not (Variables|Default|GetDead))
    (Audio|PlaySoundatLocation 0 "/Game/CharacterSounds/PlayerTakeDamageCue.PlayerTakeDamageCue" (Transformation|GetActorLocation))
    (bind _output_get (Variables|Default|Sethealth (- (Variables|Default|Gethealth) Damage)))
    (if (<= _output_get 0.0)
      (Variables|Default|Sethealth 0.0)
      (Variables|Default|SetDead true)
      (Physics|SetSimulatePhysics _firstpersonmesh true)
      (Rendering|SetVisibility _firstpersonmesh false false)
      (Class|FPSCharacter|Kill)
      (Pawn|Components|CharacterMovement|DisableMovement (Variables|Character|GetCharacterMovement))
      (Physics|SetSimulatePhysics _mesh true)
      (Rendering|SetVisibility _mesh true false))))

(event Input|MouseEvents|LeftMouseButton
  ;[1 1 1] Set attacking when pressing the attack key
  (:Pressed
    (Variables|Default|SetIsAttacking true)
    (Class|Actor|MakeNoise 1.0 0 (Transformation|GetActorLocation)))
  (:Released
    (Variables|Default|SetIsAttacking false)))

(fn ConstructionScript)