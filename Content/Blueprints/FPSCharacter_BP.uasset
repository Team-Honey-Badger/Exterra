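; First-person player character Blueprint that sets up the game HUD and tracks attack input.
; BeginPlay creates the GameHUD widget, adds it to the viewport and enables actor tick.
; Left mouse press and release toggle the IsAttacking flag.
; Noise reporting to AI for running, falling or attacking is present but disconnected, leaving Tick empty.
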(event EventBeginPlay
  ;[1 1 1] Attach HUD to player's viewport
  (bind _returnvalue (UserInterface|CreateWidget "/Game/UMG/GameHUD.GameHUD_C"))
  (UserInterface|Viewport|AddtoViewport _returnvalue 0)
  (Actor|Tick|SetActorTickEnabled true))

(event EventTick
  (params (DeltaSeconds :type Float%20%28single-precision%29))
  ;[1 1 1] Tell the AI if the character is making noise (running, jumping, or attacking)
)

(event Input|MouseEvents|LeftMouseButton
  ;[1 1 1] Set attacking when pressing the attack key
  (:Pressed
    (Variables|Default|SetIsAttacking true))
  (:Released
    (Variables|Default|SetIsAttacking false)))

(fn ConstructionScript)